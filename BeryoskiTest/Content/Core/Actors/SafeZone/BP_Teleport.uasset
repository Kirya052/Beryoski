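; BP_Teleport is a safe-zone trigger that completes the level once no enemy actors remain.
; When BP_Player enters its box in a cleared level, it saves the player's score, then opens the next level or shows the win widget with UI-only input if none exists.
; While enemies remain, an overlap shows an info widget created at BeginPlay, which is removed when the overlap ends.
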(event OnComponentEndOverlap(BoxCollision)
  (params (OverlappedComponent :type Primitive%20Component%20Object%20Reference) (OtherActor :type Actor%20Object%20Reference) (OtherComp :type Primitive%20Component%20Object%20Reference) (OtherBodyIndex :type Integer))
  ;[1 1 1] Remove info widget
  (Widget|RemovefromParent (Variables|Default|GetInfo)))

(event OnComponentBeginOverlap(BoxCollision)
  (params (OverlappedComponent :type Primitive%20Component%20Object%20Reference) (OtherActor :type Actor%20Object%20Reference) (OtherComp :type Primitive%20Component%20Object%20Reference) (OtherBodyIndex :type Integer) (bFromSweep :type Boolean) (SweepResult :type Hit%20Result%20Structure%20%28by%20ref%29))
  (bind _returnvalue (Game|GetPlayerController 0))
  ;[1 1 1] Check Enemies
  (bind _outactors (Actor|GetAllActorsOfClass "/Script/BeryoskiTest.EnemyActor"))
  (if (== (Utilities|Array|Length _outactors) 0)
    ;[1 1 1] Save score
    (bind _asbp_player (Utilities|Casting|CastToBP_Player OtherActor))
    (bind _returnvalue_2 (Class|PlayerPawn|GetScore _asbp_player))
    (Class|Teleport|SaveScore _returnvalue_2)
    (bind _returnvalue_3 (Class|Teleport|GetNextLevelName))
    (if (== _returnvalue_3 "")
      ;[1 1 1] Congratulations
      (bind _returnvalue_4 (UserInterface|CreateWidget "/Game/Core/UI/WBP_Win.WBP_Win_C"))
      (UserInterface|Viewport|AddtoViewport _returnvalue_4 0)
      (Input|SetInputModeUIOnly _returnvalue _returnvalue_4 "DoNotLock")
      (Variables|/Script/Engine.PlayerController|SetbShowMouseCursor _returnvalue true)
      (else
        ;[1 1 1] NextLevel
        (Game|OpenLevel(byName) _returnvalue_3)))
    (else
      ;[1 1 1] Add Info
      (UserInterface|Viewport|AddtoViewport (Variables|Default|GetInfo) 0))))

(event EventBeginPlay
  (bind _returnvalue (UserInterface|CreateWidget "/Game/Core/UI/WBP_Info.WBP_Info_C"))
  (Variables|Default|SetInfo _returnvalue))

(fn ConstructionScript)